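; Base visual Blueprint for long sword weapons: a non-projectile melee weapon usable on foot and on horse or camel mounts.
; BlockCollision is query-enabled only while attacking, and IsShieldActive reports that state, so the sword counts as an active shield mid-attack.
; It supplies collision boxes for Charge and Kick, and keeps the parent's combo normally while selecting mounted slashing combos for horse, rhino and camel.
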(event `self.ReceiveBeginPlay`
  (`parent.ReceiveBeginPlay`)
  (`PrimitiveComponent.SetCollisionEnabled` (`self.BlockCollision`) "NoCollision"))

(event `self.StartAttacking`
  (params (AttackType :type "/Game/Systems/Combat/SimpleAttack_AttackTypes Enum" :default "NewEnumerator0"))
  (`PrimitiveComponent.SetCollisionEnabled` (`self.BlockCollision`) "QueryOnly"))

(event `self.EndAttacking`
  (`PrimitiveComponent.SetCollisionEnabled` (`self.BlockCollision`) "NoCollision"))

(fn `CanUseWhenMounted`
  (params (Mount :type "ConanCharacter Object Reference"))
  (returns (ReturnValue :type Boolean))
  (bind _canusemounted (`/Game/Mods/MoreRealisticWeapons/WeaponSystems/FL_ComboFix.GetCanUseMountedFix` Mount true false true))
  (return _canusemounted))

(fn `GetComboType`
  (returns (Type :type "EWeaponComboType Structure"))
  (bind _combotype (`/Game/Mods/MoreRealisticWeapons/WeaponSystems/FL_ComboFix.GetComboTypeFix` (`self.CharacterOwner`) (`parent.GetComboType`) (make `EWeaponComboType` "Mounted_Slashing") (make `EWeaponComboType` "Mounted_Slashing_Rhino") (make `EWeaponComboType` "Mounted_Slashing_Camel")))
  (return _combotype))

(fn `GetSpecificCollision`
  (params (Collision :type Name))
  (returns (FoundCollision :type Boolean) (BoxExtent :type "Vector Structure") (Offset :type "Vector Structure"))
  (switch `name` Collision
    (:`Default`
      (return false (0.0 0.0 0.0) (0.0 0.0 0.0)))
    (:`Charge`
      (return true (100.0 100.0 50.0) (0.0 150.0 175.0)))
    (:`Kick`
      (return true (30.0 30.0 30.0) (0.0 0.0 0.0)))))

(fn `IsProjectile`
  (returns (ReturnValue :type Boolean))
  (return false))

(fn `IsShieldActive`
  (returns (Active :type Boolean))
  (return (`|EnumInequality` (`SceneComponent.GetCollisionEnabled` (`self.BlockCollision`)) "NoCollision")))

(fn `UserConstructionScript`
  (`parent.UserConstructionScript`))